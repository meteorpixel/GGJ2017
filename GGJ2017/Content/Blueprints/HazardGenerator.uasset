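; HazardGenerator is a spawner that places random actors from its SpawnAbleItems list, at an increasing rate over time.
; Each spawn uses the Cone component's transform with a randomized world Y, then attaches to RotatingWorld.
; BeginPlay spawns the first item, then a Tick-driven Delay repeats it at random intervals scaled by a steadily shrinking DelayMultiplier.
; SpawnWave is empty, and an older spawn chain sits disconnected.
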(event `self.ReceiveBeginPlay`
  (bind _spawnableitems (`self.SpawnAbleItems`))
  (bind (_returnvalue_location _returnvalue_rotation _returnvalue_scale) (`KismetMathLibrary.BreakTransform` (`SceneComponent.K2_GetComponentToWorld` (`self.Cone`))))
  (set `self.Delay` (* (`KismetMathLibrary.RandomFloatInRange` 0.25 0.75) (`self.DelayMultiplier`)) :!label _label)
  (bind _returnvalue (`|SpawnActorFromClass` (`KismetArrayLibrary.Array_Get` _spawnableitems (`KismetMathLibrary.RandomIntegerInRange` 0 (- (`KismetArrayLibrary.Array_Length` _spawnableitems) 1))) (`KismetMathLibrary.MakeTransform` (`KismetMathLibrary.MakeVector` (.x _returnvalue_location) (`KismetMathLibrary.RandomFloatInRange` -2000.0 2000.0) (.z _returnvalue_location)) _returnvalue_rotation _returnvalue_scale) "Undefined" "OverrideRootScale"))
  (`self.K2_AttachToActor` _returnvalue (`self.RotatingWorld`) "None" "KeepWorld" "KeepWorld" "KeepWorld" false))

(event `self.ReceiveTick`
  (params (DeltaSeconds :type "Float (single-precision)"))
  (`|ExecutionSequence`
    (:`then_0`
      (`KismetSystemLibrary.Delay` (`self.Delay`))
      (goto _label))
    (:`then_1`
      (set `self.DelayMultiplier` (- (`self.DelayMultiplier`) (/ DeltaSeconds 50.0))))))

(event `Spawn Wave`
  ;[1 1 1] Delete this?
)

(fn `UserConstructionScript`)