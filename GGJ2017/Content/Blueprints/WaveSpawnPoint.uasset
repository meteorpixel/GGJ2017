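; Wave spawn point actor that spawns a random item into a rotating world each time SpawnWave is called.
; A Cone component marks the spawn transform and is hidden at BeginPlay.
; SpawnWave picks a random class from SpawnAbleItems, spawns it at the cone and attaches it to RotatingWorld, keeping its world transform.
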(event `self.ReceiveBeginPlay`
  (`SceneComponent.SetVisibility` (`self.Cone`) false false))

(event `self.ReceiveTick`
  (params (DeltaSeconds :type "Float (single-precision)")))

(event `Spawn Wave`
  (bind _spawnableitems (`self.SpawnAbleItems`))
  (bind _returnvalue (`|SpawnActorFromClass` (`KismetArrayLibrary.Array_Get` _spawnableitems (`KismetMathLibrary.RandomIntegerInRange` 0 (- (`KismetArrayLibrary.Array_Length` _spawnableitems) 1))) (`SceneComponent.K2_GetComponentToWorld` (`self.Cone`)) "Undefined" "OverrideRootScale"))
  (set `self.MyObject` _returnvalue)
  (`/Engine/EditorBlueprintResources/StandardMacros.IsValid` (`self.MyObject`)
    (:`Is Valid`
      (`self.K2_AttachToActor` (`self.MyObject`) (`self.RotatingWorld`) "None" "KeepWorld" "KeepWorld" "KeepWorld" true))))

(fn `UserConstructionScript`)