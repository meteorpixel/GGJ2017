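; Large hazard generator that spawns random hazards at the Cone's transform with a randomized Y position, attaching each to RotatingWorld.
; BeginPlay spawns the first, then a Delay on Tick repeats the spawn at random intervals from SpawnRange scaled by DelayMultiplier.
; NextLevel steps a MultiGate through levels 2 to 5, shortening the interval and adding mines and rocks to the spawn list, with duplicate mines weighting the random pick.
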(event `NextLevel`
  ;[1 1 1] Level Up
  (`|MultiGate` false
    (:`Out 0`
      (`KismetSystemLibrary.PrintString` "Level 2" true true (struct :`R` 2.0 :`A` 1.0) 10.0)
      (set `self.SpawnRange` (1.5 1.0)))
    (:`Out 1`
      (`KismetSystemLibrary.PrintString` "Level 3" true true (struct :`R` 1.0 :`A` 1.0) 10.0)
      (set `self.SpawnRange` (1.0 0.75))
      (`KismetArrayLibrary.Array_Add` (`self.SpawnAbleItems`) "/Game/Blueprints/Hazards/Mine.Mine_C")
      (`KismetArrayLibrary.Array_Add` (`self.SpawnAbleItems`) "/Game/Blueprints/Hazards/Rocks.Rocks_C"))
    (:`Out 2`
      (`KismetSystemLibrary.PrintString` "Level 4" true true (struct :`R` 1.0 :`A` 1.0) 10.0)
      (set `self.SpawnRange` (0.75 0.5))
      (`KismetArrayLibrary.Array_Add` (`self.SpawnAbleItems`) "/Game/Blueprints/Hazards/Mine.Mine_C"))
    (:`Out 3`
      (`KismetSystemLibrary.PrintString` "Level 5" true true (struct :`R` 1.0 :`A` 1.0) 10.0)
      (set `self.SpawnRange` (0.5 0.25))
      (`KismetArrayLibrary.Array_Add` (`self.SpawnAbleItems`) "/Game/Blueprints/Hazards/Mine.Mine_C"))))

(event `self.ReceiveBeginPlay`
  (bind _spawnableitems (`self.SpawnAbleItems`))
  (bind (_returnvalue_location _returnvalue_rotation _returnvalue_scale) (`KismetMathLibrary.BreakTransform` (`SceneComponent.K2_GetComponentToWorld` (`self.Cone`))))
  (bind (_x _y) (`KismetMathLibrary.BreakVector2D` (`self.SpawnRange`)))
  ;[1 1 1] Spawen Objects
  (set `self.Delay` (* (`KismetMathLibrary.RandomFloatInRange` _x _y) (`self.DelayMultiplier`)) :!label _label)
  (bind _returnvalue (`|SpawnActorFromClass` (`KismetArrayLibrary.Array_Get` _spawnableitems (`KismetMathLibrary.RandomIntegerInRange` 0 (- (`KismetArrayLibrary.Array_Length` _spawnableitems) 1))) (`KismetMathLibrary.MakeTransform` (`KismetMathLibrary.MakeVector` (.x _returnvalue_location) (`KismetMathLibrary.RandomFloatInRange` -2000.0 2000.0) (.z _returnvalue_location)) _returnvalue_rotation _returnvalue_scale) "Undefined" "OverrideRootScale"))
  (`self.K2_AttachToActor` _returnvalue (`self.RotatingWorld`) "None" "KeepWorld" "KeepWorld" "KeepWorld" false))

(event `self.ReceiveTick`
  (params (DeltaSeconds :type "Float (single-precision)"))
  ;[1 1 1] Spawen Objects
  (`KismetSystemLibrary.Delay` (`self.Delay`))
  (goto _label))

(fn `UserConstructionScript`)