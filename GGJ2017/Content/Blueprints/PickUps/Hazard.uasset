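; Hazard pickup Blueprint that shows a configurable static mesh with an optional bobbing motion.
; The construction script applies the assigned StaticMesh to the Mesh component when it is valid.
; If AddBobbingEffect is set, BeginPlay starts a timeline that offsets the mesh locally on Z.
; Each update lerps between freshly randomized downward and upward speeds, scaled by RangeMultiplier and frame delta time.
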(event `self.ReceiveBeginPlay`
  (bind _returnvalue (* (`self.RangeMultiplier`) (`GameplayStatics.GetWorldDeltaSeconds`)))
  (if (`self.AddBobbingEffect?`)
    (bind (_direction _lerp) (`Timeline|BobbingTimeline`)
      (:`Update`
        (`SceneComponent.K2_AddLocalOffset` (`self.Mesh`) (`KismetMathLibrary.VLerp` (`KismetMathLibrary.MakeVector` 0.0 0.0 (* (`KismetMathLibrary.RandomFloatInRange` -1000.0 -500.0) _returnvalue)) (`KismetMathLibrary.MakeVector` 0.0 0.0 (* (`KismetMathLibrary.RandomFloatInRange` 500.0 1000.0) _returnvalue)) _lerp) false false)))))

(fn `UserConstructionScript`
  (bind _staticmesh (`self.StaticMesh`))
  (`/Engine/EditorBlueprintResources/StandardMacros.IsValid` _staticmesh
    (:`Is Valid`
      (`StaticMeshComponent.SetStaticMesh` (`self.Mesh`) _staticmesh))))