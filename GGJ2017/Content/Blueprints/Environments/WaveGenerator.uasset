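; WaveGenerator is an environment actor that continually spawns Wave actors at random intervals.
; Each wave takes the Cone component's transform with a randomized Y position and scale, then attaches to RotationActor keeping its world transform.
; Tick feeds a latent Delay back into the BeginPlay spawn logic, forming a repeating loop whose delay is re-randomized on every spawn.
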(event `self.ReceiveBeginPlay`
  (bind (_returnvalue_location _returnvalue_rotation _returnvalue_scale) (`KismetMathLibrary.BreakTransform` (`SceneComponent.K2_GetComponentToWorld` (`self.Cone`))))
  (set `self.Delay` (`KismetMathLibrary.RandomFloatInRange` 0.25 0.75) :!label _label)
  (bind _returnvalue (`|SpawnActorFromClass` "/Game/Blueprints/Environments/Wave.Wave_C" (`KismetMathLibrary.MakeTransform` (`KismetMathLibrary.MakeVector` (.x _returnvalue_location) (`KismetMathLibrary.RandomFloatInRange` -2000.0 2000.0) (.z _returnvalue_location)) _returnvalue_rotation (* _returnvalue_scale (`KismetMathLibrary.RandomFloatInRange` 0.5 1.5))) "Undefined" "OverrideRootScale"))
  (`self.K2_AttachToActor` _returnvalue (`self.RotationActor`) "None" "KeepWorld" "KeepWorld" "KeepWorld" false))

(event `self.ReceiveTick`
  (params (DeltaSeconds :type "Float (single-precision)"))
  (`KismetSystemLibrary.Delay` (`self.Delay`))
  (goto _label))

(fn `UserConstructionScript`)