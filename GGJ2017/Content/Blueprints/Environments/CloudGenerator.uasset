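; Cloud generator actor that keeps spawning Cloud actors at its Cone component's transform.
; Each cloud gets a randomized scale and attaches to RotationActor with world transform kept, so it follows that actor's movement.
; BeginPlay spawns the first cloud, then Tick drives a Delay node back into the same spawn chain, re-rolling a random interval of a few seconds each time.
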(event `self.ReceiveBeginPlay`
  (bind (_returnvalue_location _returnvalue_rotation _returnvalue_scale) (`KismetMathLibrary.BreakTransform` (`SceneComponent.K2_GetComponentToWorld` (`self.Cone`))))
  (set `self.Delay` (`KismetMathLibrary.RandomFloatInRange` 3.0 6.0) :!label _label)
  (bind _returnvalue (`|SpawnActorFromClass` "/Game/Blueprints/Environments/Cloud.Cloud_C" (`KismetMathLibrary.MakeTransform` _returnvalue_location _returnvalue_rotation (* _returnvalue_scale (`KismetMathLibrary.RandomFloatInRange` 0.5 1.5))) "Undefined" "OverrideRootScale"))
  (`self.K2_AttachToActor` _returnvalue (`self.RotationActor`) "None" "KeepWorld" "KeepWorld" "KeepWorld" false))

(event `self.ReceiveTick`
  (params (DeltaSeconds :type "Float (single-precision)"))
  (`KismetSystemLibrary.Delay` (`self.Delay`))
  (goto _label))

(fn `UserConstructionScript`)