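; Mine hazard Blueprint that holds logic for a vertical bobbing motion on its mesh, currently disconnected.
; BobbingTimeline's Lerp track blends random downward and upward Z offsets, scaled by RangeMultiplier and frame delta time, into an unswept local offset on Mesh each update.
; Nothing starts the timeline, and BeginPlay and the construction script are empty, so the graphs produce no movement.
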(event `self.ReceiveBeginPlay`)

(fn `UserConstructionScript`)