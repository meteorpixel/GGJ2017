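; A hazard trigger that pushes the player pawn in the direction of its Arrow component.
; On overlap it stores the world location of the pawn's BaseForMovement component and restarts a timeline.
; The timeline lerps that component from the stored location to a fixed distance along the arrow's forward vector, without sweeping, so the push ignores blocking collision.
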(event `self.Trigger.OnComponentBeginOverlap`
  (params (OverlappedComponent :type "PrimitiveComponent Object Reference") (OtherActor :type "Actor Object Reference") (OtherComp :type "PrimitiveComponent Object Reference") (OtherBodyIndex :type Integer) (bFromSweep :type Boolean) (SweepResult :type "HitResult Structure (by ref)"))
  (bind _startlocation (`self.StartLocation`))
  (bind _asplayer_pawn (cast `/Game/Blueprints/PlayerPawn` OtherActor))
  (bind _baseformovement (`/Game/Blueprints/PlayerPawn.BaseForMovement` _asplayer_pawn))
  (set `self.StartLocation` (`SceneComponent.K2_GetComponentLocation` _baseformovement))
  (bind (_direction _lerp) (`Timeline|Timeline_0` :!via `PlayFromStart`)
    (:`Update`
      (`SceneComponent.K2_SetWorldLocation` _baseformovement (`KismetMathLibrary.VLerp` _startlocation (+ _startlocation (* (`SceneComponent.GetForwardVector` (`self.Arrow`)) 400.0)) _lerp) false false))))

(fn `UserConstructionScript`)