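; Crate hazard actor that picks a random static mesh on BeginPlay and may bob it vertically.
; A separate random roll over the mesh array indices plays the bobbing timeline below 2, prints a debug string at 2, and otherwise does nothing.
; The timeline lerps between random down and up offsets, scaled by RangeMultiplier and delta time, to move the mesh locally.
; The AddBobbingEffect branch is unconnected.
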(event `self.ReceiveBeginPlay`
  (bind _staticmesh (`self.StaticMesh`))
  (bind _returnvalue (* (`self.RangeMultiplier`) (`GameplayStatics.GetWorldDeltaSeconds`)))
  (bind _returnvalue_2 (`KismetMathLibrary.RandomIntegerInRange` 0 (- (`KismetArrayLibrary.Array_Length` _staticmesh) 1)))
  (`StaticMeshComponent.SetStaticMesh` (`self.Mesh`) (`KismetArrayLibrary.Array_Get` _staticmesh _returnvalue_2))
  (`/Engine/EditorBlueprintResources/StandardMacros.CompareInt` _returnvalue_2 2
    (:`==`
      (`KismetSystemLibrary.PrintString` "Don'tBob"))
    (:`<`
      (bind (_direction _lerp) (`Timeline|BobbingTimeline`)
        (:`Update`
          (`SceneComponent.K2_AddLocalOffset` (`self.Mesh`) (`KismetMathLibrary.VLerp` (`KismetMathLibrary.MakeVector` 0.0 0.0 (* (`KismetMathLibrary.RandomFloatInRange` -1000.0 -500.0) _returnvalue)) (`KismetMathLibrary.MakeVector` 0.0 0.0 (* (`KismetMathLibrary.RandomFloatInRange` 500.0 1000.0) _returnvalue)) _lerp) false false))))))

(fn `UserConstructionScript`)