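; WaveGoverner is an actor that keeps triggering waves from a set of spawn points at random.
; Tick runs through a Delay, so roughly every 0.7 seconds it picks a random index into the SpawnPoints array.
; Its SpawnWave event casts that entry to WaveSpawnPoint and calls SpawnWave on it, leaving the spawning itself to the point.
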(event `self.ReceiveBeginPlay`)

(event `self.ReceiveTick`
  (params (DeltaSeconds :type "Float (single-precision)"))
  (`KismetSystemLibrary.Delay` 0.7)
  (`self.SpawnWave` (`KismetMathLibrary.RandomIntegerInRange` 0 (- (`KismetArrayLibrary.Array_Length` (`self.SpawnPoints`)) 1))))

(event `SpawnWave`
  (params (AtIndex :type Integer))
  (bind _aswave_spawn_point (cast `/Game/Blueprints/WaveSpawnPoint` (`KismetArrayLibrary.Array_Get` (`self.SpawnPoints`) AtIndex)))
  (`/Game/Blueprints/WaveSpawnPoint.Spawn Wave` _aswave_spawn_point))

(fn `UserConstructionScript`)