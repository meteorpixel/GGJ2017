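; MenuController is a Blueprint that creates the MainMenu widget on BeginPlay and drives it with the space bar alone.
; Pressing Space opens a gate and starts a one-second retriggerable delay, so holding through the delay calls SelectOption.
; Every release closes the gate and calls NextButton, including after a long-press selection.
; Print strings trace these actions, and the Enter key only prints a debug message.
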(event `self.ReceiveBeginPlay`
  (`KismetSystemLibrary.PrintString` "Hello")
  (bind _returnvalue (`|CreateWidget` "/Game/GUI/MainMenu.MainMenu_C" (`GameplayStatics.GetPlayerController` 0)))
  (set `self.MainMenu` _returnvalue)
  (`UserWidget.AddToViewport` (`self.MainMenu`) 0))

(event `Key|Enter`
  (params (Key :type "Key Structure" :default "AnyKey"))
  (:`Pressed`
    (`KismetSystemLibrary.PrintString` "Hello")))

(event `Key|SpaceBar`
  (params (Key :type "Key Structure" :default "AnyKey"))
  (:`Pressed`
    (`|ExecutionSequence`
      (:`then_0`
        (`KismetSystemLibrary.RetriggerableDelay` 1.0)
        (`/Engine/EditorBlueprintResources/StandardMacros.Gate` true :!label _label
          (:`Exit`
            (`KismetSystemLibrary.PrintString` "Select")
            (`/Game/GUI/MainMenu.SelectOption` (`self.MainMenu`)))))
      (:`then_1`
        (goto _label :!via `Open`))))
  (:`Released`
    (`|ExecutionSequence`
      (:`then_0`
        (goto _label :!via `Close`))
      (:`then_1`
        (`/Game/GUI/MainMenu.NextButton` (`self.MainMenu`))
        (`KismetSystemLibrary.PrintString` "Next")))))

(fn `UserConstructionScript`)