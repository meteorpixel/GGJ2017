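; Game-over screen controller that creates the GameOver widget on BeginPlay and drives its menu with the Space Bar alone.
; Pressing starts a one-second retriggerable delay and opens a gate, so holding until it elapses calls SelectOption.
; Releasing closes the gate, cancelling a pending selection, and always calls NextOption, even after a hold has selected.
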(event `self.ReceiveBeginPlay`
  (`KismetSystemLibrary.PrintString` "Hello")
  (bind _returnvalue (`|CreateWidget` "/Game/GUI/GameOver.GameOver_C"))
  (set `self.GameOverScreen` _returnvalue)
  (`UserWidget.AddToViewport` (`self.GameOverScreen`) 0))

(event `Key|SpaceBar` :consume false
  (params (Key :type "Key Structure" :default "AnyKey"))
  (:`Pressed`
    (`|ExecutionSequence`
      (:`then_0`
        (`KismetSystemLibrary.RetriggerableDelay` 1.0)
        (`/Engine/EditorBlueprintResources/StandardMacros.Gate` true :!label _label
          (:`Exit`
            (`KismetSystemLibrary.PrintString` "Select")
            (`/Game/GUI/GameOver.SelectOption` (`self.GameOverScreen`)))))
      (:`then_1`
        (goto _label :!via `Open`))))
  (:`Released`
    (`|ExecutionSequence`
      (:`then_0`
        (goto _label :!via `Close`))
      (:`then_1`
        (`KismetSystemLibrary.PrintString` "Next")
        (`/Game/GUI/GameOver.NextOption` (`self.GameOverScreen`))))))

(fn `UserConstructionScript`)