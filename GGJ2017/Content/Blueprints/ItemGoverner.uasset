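; ItemGoverner periodically triggers item waves at randomly chosen spawn points while it is enabled.
; Tick feeds a one-second Delay, which acts as a repeating timer because calls made during the wait are ignored.
; After each delay it picks a random SpawnPoints index, and its SpawnWave event casts that entry to ItemGenerator and calls SpawnWave on it.
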(event `self.ReceiveBeginPlay`)

(event `self.ReceiveTick`
  (params (DeltaSeconds :type "Float (single-precision)"))
  (if (`self.Enabled`)
    (`KismetSystemLibrary.Delay` 1.0)
    (`self.SpawnWave` (`KismetMathLibrary.RandomIntegerInRange` 0 (- (`KismetArrayLibrary.Array_Length` (`self.SpawnPoints`)) 1)))))

(event `SpawnWave`
  (params (AtIndex :type Integer))
  (bind _asitem_generator (cast `/Game/Blueprints/ItemGenerator` (`KismetArrayLibrary.Array_Get` (`self.SpawnPoints`) AtIndex)))
  (`/Game/Blueprints/ItemGenerator.Spawn Wave` _asitem_generator))

(fn `UserConstructionScript`)