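; Player pawn for a one-button game that steers side to side along Y with Space.
; Holding Space plays a timeline and releasing reverses it, blending velocity and tilt between two extremes while Tick applies the offset.
; Board overlaps with "Destroy"-tagged components stop Tick and reload the current level after a short delay.
; A Collected event increments and prints the score.
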(event `Key|SpaceBar`
  (params (Key :type "Key Structure" :default "AnyKey"))
  ;[1 1 1] Pawn Direction
  (:`Pressed`
    (bind (_direction _lerp) (`Timeline|PawnDirectionTimeline` :!label _label)
      (:`Update`
        (set `self.PawnDirection` (`KismetMathLibrary.VLerp` (0.0 300.0 0.0) (0.0 -300.0 0.0) _lerp))
        (`SceneComponent.K2_SetRelativeRotation` (`self.BaseForMovement`) (`KismetMathLibrary.RLerp` (struct :`Yaw` 30.0 :`Roll` 30.0) (struct :`Yaw` -30.0 :`Roll` -30.0) _lerp true) false false))))
  (:`Released`
    (goto _label :!via `Reverse`)))

(event `self.ReceiveBeginPlay`
  ;[1 1 1] Pawn Direction
  (`TimelineComponent.SetPlaybackPosition` (`self.PawnDirectionTimeline`) 0.5 false true)
  (goto _label :!via `Reverse`))

(event `self.ReceiveTick`
  (params (DeltaSeconds :type "Float (single-precision)"))
  ;[1 1 1] Pawn Movement
  (`SceneComponent.K2_AddWorldOffset` (`self.BaseForMovement`) (* (`self.PawnDirection`) (`GameplayStatics.GetWorldDeltaSeconds`)) false false))

(event `self.Board.OnComponentBeginOverlap`
  (params (OverlappedComponent :type "PrimitiveComponent Object Reference") (OtherActor :type "Actor Object Reference") (OtherComp :type "PrimitiveComponent Object Reference") (OtherBodyIndex :type Integer) (bFromSweep :type Boolean) (SweepResult :type "HitResult Structure (by ref)"))
  ;[1 1 1] Overlap
  (if (`ActorComponent.ComponentHasTag` OtherComp "Destroy")
    (`self.SetActorTickEnabled` false)
    (`KismetSystemLibrary.PrintString` "Destroy")
    (`KismetSystemLibrary.Delay` 1.0)
    (bind _returnvalue (`GameplayStatics.GetCurrentLevelName` true))
    (`GameplayStatics.OpenLevel` (`KismetStringLibrary.Conv_StringToName` _returnvalue))
    (else
      (`KismetSystemLibrary.PrintString` "Hello"))))

(event `Collected`
  ;[1 1 1] Collectible
  (bind _result (`/Engine/EditorBlueprintResources/StandardMacros.IncrementInt` (`self.Collectibles`))
    (:`  `
      (`KismetSystemLibrary.PrintString` (`KismetStringLibrary.Concat_StrStr` "Score = " (`KismetStringLibrary.Conv_IntToString` _result))))))

(fn `UserConstructionScript`)