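; BuoyGenerator is an actor that continually spawns MarkerBuoy actors at its Cone component's world transform.
; Each Tick runs through a randomized delay scaled down by SpeedMultiplier, which is refreshed from the RotationalWorld2 actor's RotationalSpeed, so spawn rate follows world rotation speed.
; Each new buoy is attached to RotationActor with world transform kept, so it moves with the rotating world.
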(event `self.ReceiveTick`
  (params (DeltaSeconds :type "Float (single-precision)"))
  (`KismetSystemLibrary.Delay` (/ (`KismetMathLibrary.RandomFloatInRange` 0.5 0.6) (`self.SpeedMultiplier`)))
  (`|ExecutionSequence`
    (:`then_0`
      (bind _asrotational_world_2 (cast `/Game/Blueprints/RotationalWorld2` (`self.RotationActor`)))
      (set `self.SpeedMultiplier` (/ (`/Game/Blueprints/RotationalWorld2.RotationalSpeed` _asrotational_world_2) 10.0)))
    (:`then_1`
      (bind _returnvalue (`|SpawnActorFromClass` "/Game/Blueprints/MarkerBuoy.MarkerBuoy_C" (`SceneComponent.K2_GetComponentToWorld` (`self.Cone`)) "Undefined" "OverrideRootScale"))
      (`self.K2_AttachToActor` _returnvalue (`self.RotationActor`) "None" "KeepWorld" "KeepWorld" "KeepWorld" false))))

(fn `UserConstructionScript`)